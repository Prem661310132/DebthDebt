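; Fishing spot Blueprint that runs a round-based reeling minigame through a UMG widget it creates and passes itself to.
; AsMinigameSetup supplies each round's value, speed, duration and failure penalty.
; A timer event drains the widget's progress bar, and MinigameFailed adds a fraction of the round's duration to elapsed time.
; Winning advances the round or removes the widget, while losing resets state and ends the minigame.
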(event Custom|MinigameWon
  (bind _as_minigamesetup (Variables|Default|GetAs%20MinigameSetup))
  (bind _returnvalue (Utilities|Array|Length _as_minigamesetup))
  ;[0.15 0.15 0.15 0.5] On Minigame on success Round Increase
  (if (> _returnvalue 1)
    (if (>= (Variables|Default|GetCurrentRound) (- _returnvalue 0))
      (Widget|RemovefromParent (Variables|Default|GetAs%20UMG_MinigameUI) :!label _label)
      (else
        (bind _result (Math|Integer|IncrementInt (Variables|Default|GetCurrentRound))
          (:%20%20
            (CallFunction|SetRound _result)))))
    (else
      (goto _label))))

(event Custom|MinigameFailed
  (bind _as_minigamesetup (Variables|Default|GetAs%20MinigameSetup))
  (bind _currentround (Variables|Default|GetCurrentRound))
  (bind _output (Utilities|Array|Get(acopy) _as_minigamesetup _currentround))
  ;[0.15 0.15 0.15 0.5] MinigameFailed Decrease Timer
  (Variables|Default|SetElapseTime (+ (Variables|Default|GetElapseTime) (* (.duration _output) (.faileddecrement _output)))))

(event Custom|Set%20Round
  (params (Round :type Integer))
  (bind _as_minigamesetup (Variables|Default|GetAs%20MinigameSetup))
  (bind _output (Utilities|Array|Get(acopy) _as_minigamesetup Round))
  ;[0.15 0.15 0.15 0.5] Set New Round and Deplete Progress Bar
  (Variables|Default|SetCurrentRound Round)
  (Default|StartRound (Variables|Default|GetAs%20UMG_MinigameUI) (.value _output) (.speed _output))
  (if (Utilities|Time|IsValidTimerHandle (Variables|Default|GetMinigameTimer))
    (Utilities|Time|ClearandInvalidateTimerbyHandle (Variables|Default|GetMinigameTimer))
    (bind _returnvalue (Utilities|Time|SetTimerbyEvent (delegate Custom|DepleteTimer) 0.02))
    (Variables|Default|SetMinigameTimer _returnvalue)
    (Progress|SetPercent (Variables|/Game/Fishing/UMG_MinigameUI.UMG_MinigameUI_C|GetTimerBar (Variables|Default|GetAs%20UMG_MinigameUI)) 0.0)
    (Variables|Default|SetElapseTime 0.0)
    (Variables|Default|SetCurrentTime 1.0)))

(event Custom|DepleteTimer
  (bind _minigametimer (Variables|Default|GetMinigameTimer))
  ;[0.15 0.15 0.15 0.5] Set New Round and Deplete Progress Bar
  (bind _output_get (Variables|Default|SetElapseTime (+ (Variables|Default|GetElapseTime) 0.02)))
  (Progress|SetPercent (Variables|/Game/Fishing/UMG_MinigameUI.UMG_MinigameUI_C|GetTimerBar (Variables|Default|GetAs%20UMG_MinigameUI)) (- (Variables|Default|GetCurrentTime) (/ _output_get (.duration (Utilities|Array|Get(acopy) (Variables|Default|GetAs%20MinigameSetup) (Variables|Default|GetCurrentRound))))))
  (if (<= (Variables|/Script/UMG.ProgressBar|GetPercent (Variables|/Game/Fishing/UMG_MinigameUI.UMG_MinigameUI_C|GetTimerBar (Variables|Default|GetAs%20UMG_MinigameUI))) 0.0)
    (if (Utilities|Time|IsValidTimerHandle _minigametimer)
      (Utilities|Time|ClearandInvalidateTimerbyHandle _minigametimer)
      (CallFunction|MinigameFailed))))

(event Custom|MinigameLost
  ;[0.15 0.15 0.15 0.5] GameLost Reset Variable
  (Utilities|FlowControl|Sequence
    (:then_0
      (Variables|Default|SetCurrentRound 0)
      (Variables|Default|SetElapseTime 0.0)
      (Variables|Default|SetCurrentTime 1.0))
    (:then_1
      (Default|EndFishingMinigame (Variables|Default|GetAs%20UMG_MinigameUI)))))

(event Custom|OnMinigameInteract
  (if (Variables|Default|GetisReadytoReel)
    (Default|OnMinigameInteracted (Variables|Default|GetAs%20UMG_MinigameUI))))

(event Custom|StartMinigame
  ;[0.15 0.15 0.15 0.5] Start Minigame set round add widget
  (bind _returnvalue (UserInterface|CreateWidget "/Game/Fishing/UMG_MinigameUI.UMG_MinigameUI_C" 0 self))
  (bind _output_get (Variables|Default|SetAs%20UMG_MinigameUI _returnvalue))
  (UserInterface|Viewport|AddtoViewport _output_get 0)
  (Variables|Default|SetisReadytoReel true)
  (CallFunction|SetRound))

(fn ConstructionScript)