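; BP_FishSpot is a fishing spot actor that populates a box-shaped zone with fish.
; The construction script sizes the FishingZone box from FishingZoneRange.
; BeginPlay spawns NoOfFish actors of FishType at random points within the box bounds, each with a random roll-free rotation, adjusting for collisions but always spawning.
; A note in the graph flags the random spawning as needing a fix.
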(event EventBeginPlay
  (bind _fishingzone (Variables|Default|GetFishingZone))
  (bind (_origin _boxextent) (Collision|GetComponentBounds _fishingzone))
  ;[0.15 0.15 0.15 0.5] Random spawn fish in zone \\ Need Fix
  (for _index (range 0 (- (Variables|Setting|GetNoOfFish) 1))
    (Game|SpawnActorfromClass (Variables|Setting|GetFishType) (Math|Transform|MakeTransform (Math|Random|RandomPointinBoundingBox _origin _boxextent) (Math|Random|RandomRotator false)) "AdjustIfPossibleButAlwaysSpawn" "MultiplyWithRoot" 0 0)))

(fn ConstructionScript
  (Components|Box|SetBoxExtent (Variables|Default|GetFishingZone) (Variables|Setting|GetFishingZoneRange) true))