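; Day-cycle manager for the fishing game: runs a five-day countdown, then plays a good or bad debt ending cutscene.
; Tick drains time while undocked, scaled when fishing, and lerps sun, skylight and fog from it, toggling clouds.
; SkipTime fast-forwards the clock by timeline.
; Day rollover saves progress, moves the player to the dock and resets fish spots; ending undocked also costs money and clears inventory.
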(event Custom|StartNewDay
  (params (RestedDock :type Actor%20Object%20Reference))
  (bind _returnvalue (Game|GetPlayerCameraManager 0))
  ;[0.15 0.15 0.15 0.5] NewDay
  (CameraFades|StartCameraFade _returnvalue 0.0 1.0 4.0 "(R=0.000000,G=0.000000,B=0.000000,A=1.000000)" false false)
  (Variables|Cycle|SetTimeRemaining (Variables|Cycle|GetTimePerDay))
  (bind _asbp_player_ship_character (Utilities|Casting|CastToBP_PlayerShipCharacter (Game|GetPlayerCharacter 0)))
  (bind _returnvalue_2 (SaveGame|CreateSaveGameObject "/Game/DayManager/BP_MySaveGame.BP_MySaveGame_C"))
  (Variables|/Game/DayManager/BP_MySaveGame.BP_MySaveGame_C|SetSavedMoney _returnvalue_2 (Variables|/Game/Currency/AC_MoneyManager.AC_MoneyManager_C|GetCurrentMoney (Variables|/Game/ThirdPerson/Blueprints/BP_PlayerShipCharacter.BP_PlayerShipCharacter_C|GetAC_MoneyManager _asbp_player_ship_character)))
  (Variables|/Game/DayManager/BP_MySaveGame.BP_MySaveGame_C|SetSavedRodTier _returnvalue_2 (Variables|/Game/ThirdPerson/Blueprints/BP_PlayerShipCharacter.BP_PlayerShipCharacter_C|GetFishingRodTier _asbp_player_ship_character))
  (Variables|/Game/DayManager/BP_MySaveGame.BP_MySaveGame_C|SetSavedEngineTier _returnvalue_2 (Variables|/Game/ThirdPerson/Blueprints/BP_PlayerShipCharacter.BP_PlayerShipCharacter_C|GetEngineTier _asbp_player_ship_character))
  (Variables|/Game/DayManager/BP_MySaveGame.BP_MySaveGame_C|SetSavedStorageTier _returnvalue_2 (Variables|/Game/ThirdPerson/Blueprints/BP_PlayerShipCharacter.BP_PlayerShipCharacter_C|GetStorageTier _asbp_player_ship_character))
  (Variables|/Game/DayManager/BP_MySaveGame.BP_MySaveGame_C|SetSavedDeepWaterRod _returnvalue_2 (Variables|/Game/ThirdPerson/Blueprints/BP_PlayerShipCharacter.BP_PlayerShipCharacter_C|GetHasDeepWaterRod _asbp_player_ship_character))
  (Variables|/Game/DayManager/BP_MySaveGame.BP_MySaveGame_C|SetSavedMangroveRod _returnvalue_2 (Variables|/Game/ThirdPerson/Blueprints/BP_PlayerShipCharacter.BP_PlayerShipCharacter_C|GetHasMangroveRod _asbp_player_ship_character))
  (Variables|/Game/DayManager/BP_MySaveGame.BP_MySaveGame_C|SetSavedInventory _returnvalue_2 (Variables|/Game/Inventory/AC_Inventory.AC_Inventory_C|GetInventory (Variables|/Game/ThirdPerson/Blueprints/BP_PlayerShipCharacter.BP_PlayerShipCharacter_C|GetAC_Inventory _asbp_player_ship_character)))
  (Variables|/Game/DayManager/BP_MySaveGame.BP_MySaveGame_C|SetSavedInventoryState _returnvalue_2 (Variables|/Game/Inventory/AC_Inventory.AC_Inventory_C|GetInventoryState (Variables|/Game/ThirdPerson/Blueprints/BP_PlayerShipCharacter.BP_PlayerShipCharacter_C|GetAC_Inventory _asbp_player_ship_character)))
  (SaveGame|SaveGametoSlot _returnvalue_2 "MySaveSlot")
  (Transformation|SetActorLocation (Game|Player|GetPlayerPawn 0) (Transformation|GetActorLocation RestedDock) false true)
  (CameraFades|StartCameraFade :self _returnvalue :FromAlpha 1.0 :Duration 4.0)
  (bind _outactors (Actor|GetAllActorsOfClass "/Game/Fishing/BP_FishSpot.BP_FishSpot_C"))
  (for _array_element _outactors
    (Default|ResetFishCount _array_element)))

(event Custom|EndGame
  (bind _as_bp_player_ship_character (Variables|Default|GetAs%20BP%20Player%20Ship%20Character))
  (bind _ac_moneymanager (Variables|/Game/ThirdPerson/Blueprints/BP_PlayerShipCharacter.BP_PlayerShipCharacter_C|GetAC_MoneyManager _as_bp_player_ship_character))
  ;[0.15 0.15 0.15 0.5] Endgame
  (if (Default|HasEnoughMoney _ac_moneymanager 3000)
    (Default|RemoveMoney _ac_moneymanager (Variables|Cycle|GetDebt))
    (Development|PrintString "Your Debt is paid" true true "(R=0.178592,G=1.000000,B=0.003301,A=1.000000)" 5.0)
    (bind _returnvalue (UserInterface|CreateWidget "/Game/Cutscene/UMG_Cutscene.UMG_Cutscene_C"))
    (UserInterface|Viewport|AddtoViewport _returnvalue 0)
    (Default|PlayGoodEnd _returnvalue)
    (else
      (Default|RemoveMoney _ac_moneymanager (Variables|/Game/Currency/AC_MoneyManager.AC_MoneyManager_C|GetCurrentMoney _ac_moneymanager))
      (Development|PrintString "You lose" true true "(R=1.000000,G=0.000000,B=0.986207,A=1.000000)" 5.0)
      (bind _returnvalue_2 (UserInterface|CreateWidget "/Game/Cutscene/UMG_Cutscene.UMG_Cutscene_C"))
      (UserInterface|Viewport|AddtoViewport _returnvalue_2 0)
      (Default|PlayBadEnd _returnvalue_2))))

(event Custom|FailedNewDay
  (bind _returnvalue (Game|GetPlayerCameraManager 0))
  (bind _dock (Variables|Default|GetDock))
  ;[0.15 0.15 0.15 0.5] NewDay
  (CameraFades|StartCameraFade _returnvalue 0.0 1.0 4.0 "(R=0.000000,G=0.000000,B=0.000000,A=1.000000)" false false)
  (Variables|Cycle|SetTimeRemaining (Variables|Cycle|GetTimePerDay))
  (bind _asbp_player_ship_character (Utilities|Casting|CastToBP_PlayerShipCharacter (Game|GetPlayerCharacter 0)))
  (bind _returnvalue_2 (SaveGame|CreateSaveGameObject "/Game/DayManager/BP_MySaveGame.BP_MySaveGame_C"))
  (Default|RemoveMoney (Variables|/Game/ThirdPerson/Blueprints/BP_PlayerShipCharacter.BP_PlayerShipCharacter_C|GetAC_MoneyManager _asbp_player_ship_character) 100)
  (Variables|/Game/DayManager/BP_MySaveGame.BP_MySaveGame_C|SetSavedMoney _returnvalue_2 (Variables|/Game/Currency/AC_MoneyManager.AC_MoneyManager_C|GetCurrentMoney (Variables|/Game/ThirdPerson/Blueprints/BP_PlayerShipCharacter.BP_PlayerShipCharacter_C|GetAC_MoneyManager _asbp_player_ship_character)))
  (Variables|/Game/DayManager/BP_MySaveGame.BP_MySaveGame_C|SetSavedRodTier _returnvalue_2 (Variables|/Game/ThirdPerson/Blueprints/BP_PlayerShipCharacter.BP_PlayerShipCharacter_C|GetFishingRodTier _asbp_player_ship_character))
  (Variables|/Game/DayManager/BP_MySaveGame.BP_MySaveGame_C|SetSavedEngineTier _returnvalue_2 (Variables|/Game/ThirdPerson/Blueprints/BP_PlayerShipCharacter.BP_PlayerShipCharacter_C|GetEngineTier _asbp_player_ship_character))
  (Variables|/Game/DayManager/BP_MySaveGame.BP_MySaveGame_C|SetSavedStorageTier _returnvalue_2 (Variables|/Game/ThirdPerson/Blueprints/BP_PlayerShipCharacter.BP_PlayerShipCharacter_C|GetStorageTier _asbp_player_ship_character))
  (Variables|/Game/DayManager/BP_MySaveGame.BP_MySaveGame_C|SetSavedDeepWaterRod _returnvalue_2 (Variables|/Game/ThirdPerson/Blueprints/BP_PlayerShipCharacter.BP_PlayerShipCharacter_C|GetHasDeepWaterRod _asbp_player_ship_character))
  (Variables|/Game/DayManager/BP_MySaveGame.BP_MySaveGame_C|SetSavedMangroveRod _returnvalue_2 (Variables|/Game/ThirdPerson/Blueprints/BP_PlayerShipCharacter.BP_PlayerShipCharacter_C|GetHasMangroveRod _asbp_player_ship_character))
  (Utilities|Map|Clear (Variables|/Game/Inventory/AC_Inventory.AC_Inventory_C|GetInventory (Variables|/Game/ThirdPerson/Blueprints/BP_PlayerShipCharacter.BP_PlayerShipCharacter_C|GetAC_Inventory _asbp_player_ship_character)))
  (Utilities|Map|Clear (Variables|/Game/Inventory/AC_Inventory.AC_Inventory_C|GetInventoryState (Variables|/Game/ThirdPerson/Blueprints/BP_PlayerShipCharacter.BP_PlayerShipCharacter_C|GetAC_Inventory _asbp_player_ship_character)))
  (Variables|/Game/DayManager/BP_MySaveGame.BP_MySaveGame_C|SetSavedInventory _returnvalue_2 (Variables|/Game/Inventory/AC_Inventory.AC_Inventory_C|GetInventory (Variables|/Game/ThirdPerson/Blueprints/BP_PlayerShipCharacter.BP_PlayerShipCharacter_C|GetAC_Inventory _asbp_player_ship_character)))
  (Variables|/Game/DayManager/BP_MySaveGame.BP_MySaveGame_C|SetSavedInventoryState _returnvalue_2 (Variables|/Game/Inventory/AC_Inventory.AC_Inventory_C|GetInventoryState (Variables|/Game/ThirdPerson/Blueprints/BP_PlayerShipCharacter.BP_PlayerShipCharacter_C|GetAC_Inventory _asbp_player_ship_character)))
  (SaveGame|SaveGametoSlot _returnvalue_2 "MySaveSlot")
  (Transformation|SetActorLocation (Game|Player|GetPlayerPawn 0) (Transformation|GetActorLocation _dock) false true)
  (CameraFades|StartCameraFade :self _returnvalue :FromAlpha 1.0 :Duration 4.0)
  (Default|InstantDocking _dock)
  (bind _outactors (Actor|GetAllActorsOfClass "/Game/Fishing/BP_FishSpot.BP_FishSpot_C"))
  (for _array_element _outactors
    (Default|ResetFishCount _array_element)))

(event Custom|StopEverything
  (bind _as_bp_player_ship_character (Variables|Default|GetAs%20BP%20Player%20Ship%20Character))
  (if (Variables|/Game/ThirdPerson/Blueprints/BP_PlayerShipCharacter.BP_PlayerShipCharacter_C|GetIsFishing (Variables|Default|GetAs%20BP%20Player%20Ship%20Character))
    (Default|PlayerEndMinigame _as_bp_player_ship_character))
  (Default|ClosedInventoryBeforeInteract (Variables|/Game/ThirdPerson/Blueprints/BP_PlayerShipCharacter.BP_PlayerShipCharacter_C|GetAC_Inventory _as_bp_player_ship_character))
  (Variables|Cycle|SetTimeRemaining 0.0))

(event Custom|SkipTime
  (bind _as_bp_player_ship_character (Variables|Default|GetAs%20BP%20Player%20Ship%20Character))
  ;[0.15 0.15 0.15 0.5] Day Time
  (bind _returnvalue (Audio|SpawnSound2D "/Game/Sound/SFX/FastClock.FastClock" 1.0 1.0 0.0 0))
  (Variables|TimeSkip|SetClockSound _returnvalue)
  (Variables|TimeSkip|SetStartSkipTime (Variables|Cycle|GetTimeRemaining))
  (bind _newtrack_0 (Timeline|TimeSkip_Timeline PlayFromStart)
    (:Update
      (Variables|Cycle|SetTimeRemaining (Math|Float|Lerp (Variables|TimeSkip|GetStartSkipTime) 0.0 _newtrack_0)))
    (:Finished
      (Audio|Components|Audio|Stop (Variables|TimeSkip|GetClockSound))
      (if (<= (Variables|Cycle|GetTimeRemaining) 0.0)
        (Variables|Cycle|SetCurrentDay (+ (Variables|Cycle|GetCurrentDay) 1))
        (if (> (Variables|Cycle|GetCurrentDay) 5)
          (Utilities|FlowControl|DoOnce false
            (:Completed
              (CallFunction|StopEverything)
              (CallFunction|EndGame)))
          (elif (Variables|/Game/ThirdPerson/Blueprints/BP_PlayerShipCharacter.BP_PlayerShipCharacter_C|GetIsDocked _as_bp_player_ship_character)
            (CallFunction|StartNewDay (Variables|Default|GetDock))
            (elif (Variables|/Game/ThirdPerson/Blueprints/BP_PlayerShipCharacter.BP_PlayerShipCharacter_C|GetIsFishing _as_bp_player_ship_character)
              (Default|PlayerEndMinigame (Variables|Default|GetAs%20BP%20Player%20Ship%20Character))
              (CallFunction|FailedNewDay)
              (else
                (CallFunction|FailedNewDay)))))))))

(event Custom|setRestedDock
  (params (Dock :type BP%20Dock%20Object%20Reference))
  ;[0.15 0.15 0.15 0.5] Day Time
  (Variables|Default|SetDock Dock))

(event EventBeginPlay
  ;[0.15 0.15 0.15 0.5] Start
  (bind _asbp_player_ship_character (Utilities|Casting|CastToBP_PlayerShipCharacter (Game|GetPlayerCharacter 0)))
  (Variables|Default|SetAs%20BP%20Player%20Ship%20Character _asbp_player_ship_character)
  (Variables|Cycle|SetTimeRemaining (Variables|Cycle|GetTimePerDay))
  (bind _returnvalue (UserInterface|CreateWidget "/Game/DayManager/WBP_GameHUD.WBP_GameHUD_C"))
  (UserInterface|Viewport|AddtoViewport _returnvalue 0))

(event EventTick
  (params (DeltaSeconds :type Float%20%28single-precision%29))
  (bind _returnvalue (Utilities|Time|GetWorldDeltaSeconds))
  (bind _as_bp_player_ship_character (Variables|Default|GetAs%20BP%20Player%20Ship%20Character))
  (bind _mainsun (Variables|Environtment|GetMainSun))
  (bind _mainfog (Variables|Environtment|GetMainFog))
  (bind _as_bp_player_ship_character_2 (Variables|Default|GetAs%20BP%20Player%20Ship%20Character))
  (bind _skylight (Variables|Environtment|GetSkyLight))
  (bind _lightcomponent (Variables|/Script/Engine.Light|GetLightComponent _mainsun))
  (bind _component (Variables|/Script/Engine.ExponentialHeightFog|GetComponent _mainfog))
  (bind _lightcomponent_2 (Variables|/Script/Engine.SkyLight|GetLightComponent _skylight))
  ;[0.15 0.15 0.15 0.5] Day Time
  (if (not (Variables|/Game/ThirdPerson/Blueprints/BP_PlayerShipCharacter.BP_PlayerShipCharacter_C|GetIsDocked _as_bp_player_ship_character))
    (Variables|Cycle|SetTimeRemaining (- (Variables|Cycle|GetTimeRemaining) (Math|Float|SelectFloat (* _returnvalue (Variables|/Game/ThirdPerson/Blueprints/BP_PlayerShipCharacter.BP_PlayerShipCharacter_C|GetFishingMultiplyer _as_bp_player_ship_character)) _returnvalue (Variables|/Game/ThirdPerson/Blueprints/BP_PlayerShipCharacter.BP_PlayerShipCharacter_C|GetIsFishing _as_bp_player_ship_character))))
    (Utilities|FlowControl|Sequence
      (:then_0
        (if (<= (Variables|Cycle|GetTimeRemaining) 0.0)
          (Variables|Cycle|SetCurrentDay (+ (Variables|Cycle|GetCurrentDay) 1))
          (if (> (Variables|Cycle|GetCurrentDay) 5)
            (Utilities|FlowControl|DoOnce false
              (:Completed
                (CallFunction|StopEverything)
                (CallFunction|EndGame)))
            (elif (Variables|/Game/ThirdPerson/Blueprints/BP_PlayerShipCharacter.BP_PlayerShipCharacter_C|GetIsDocked _as_bp_player_ship_character_2)
              (CallFunction|StartNewDay (Variables|Default|GetDock))
              (elif (Variables|/Game/ThirdPerson/Blueprints/BP_PlayerShipCharacter.BP_PlayerShipCharacter_C|GetIsFishing _as_bp_player_ship_character_2)
                (Default|PlayerEndMinigame (Variables|Default|GetAs%20BP%20Player%20Ship%20Character))
                (CallFunction|FailedNewDay)
                (else
                  (CallFunction|FailedNewDay)))))))
      (:then_1
        (Rendering|Components|Light|SetIntensity _lightcomponent (Math|Float|Lerp 2.0 0.04 (Math|Float|MapRangeClamped (Variables|Cycle|GetTimeRemaining) 3e+02 2.4e+02 0.0 1.0)))
        (Class|LightComponent|SetTemperature _lightcomponent (Math|Float|Lerp 3.5e+03 5.5e+03 (Math|Float|MapRangeClamped (Variables|Cycle|GetTimeRemaining) 3e+02 2.4e+02 0.0 1.0)))
        (Rendering|Components|Light|SetLightColor _lightcomponent (Math|Color|Lerp(LinearColor) "(R=1.000000,G=1.000000,B=1.000000,A=1.000000)" "(R=0.564706,G=0.972549,B=1.000000,A=1.000000)" (Math|Float|MapRangeClamped (Variables|Cycle|GetTimeRemaining) 3e+02 2.4e+02 0.0 1.0)) true)
        (Class|ExponentialHeightFogComponent|SetFogDensity _component (Math|Float|Lerp 0.05 0.07 (Math|Float|MapRangeClamped (Variables|Cycle|GetTimeRemaining) 3e+02 2.4e+02 0.0 1.0)))
        (Class|ExponentialHeightFogComponent|SetFogInscatteringColor _component (Math|Color|Lerp(LinearColor) :A "(R=0.474510,G=0.572549,B=1.000000,A=1.000000)" :Alpha (Math|Float|MapRangeClamped (Variables|Cycle|GetTimeRemaining) 3e+02 2.4e+02 0.0 1.0)))
        (Class|ExponentialHeightFogComponent|SetVolumetricFogExtinctionScale _component (Math|Float|Lerp 4.0 6.0 (Math|Float|MapRangeClamped (Variables|Cycle|GetTimeRemaining) 3e+02 2.4e+02 0.0 1.0)))
        (Rendering|Components|Light|SetLightColor _lightcomponent_2 (Math|Color|Lerp(LinearColor) "(R=1.000000,G=1.000000,B=1.000000,A=1.000000)" "(R=0.666667,G=0.698039,B=1.000000,A=1.000000)" (Math|Float|MapRangeClamped (Variables|Cycle|GetTimeRemaining) 3e+02 2.4e+02 0.0 1.0)))
        (Rendering|Components|Light|SetIntensity _lightcomponent_2 (Math|Float|Lerp 1.0 0.2 (Math|Float|MapRangeClamped (Variables|Cycle|GetTimeRemaining) 3e+02 2.4e+02 0.0 1.0)))
        (if (> (/ (Variables|Cycle|GetTimeRemaining) (Variables|Cycle|GetTimePerDay)) 0.3)
          (Rendering|SetVisibility (Variables|/Script/Engine.VolumetricCloud|GetVolumetricCloudComponent (Variables|Environtment|GetVolumnCloud)) true false)
          (else
            (Rendering|SetVisibility (Variables|/Script/Engine.VolumetricCloud|GetVolumetricCloudComponent (Variables|Environtment|GetVolumnCloud)) false false)))))))

(fn ConstructionScript)

(fn GetFormattedTimeOfDay
  (bind _timeperday (Variables|Cycle|GetTimePerDay))
  (bind _timeremaining (Variables|Cycle|GetTimeRemaining))
  (bind _returnvalue (- _timeperday _timeremaining))
  (bind _returnvalue_2 (* _returnvalue 2.0))
  (bind _returnvalue_3 (+ 2.4e+02 _returnvalue_2))
  (bind _returnvalue_4 (/ _returnvalue_3 6e+01))
  (return (Utilities|Text|FormatText "{HH}:{MM}" (Utilities|Text|ToText(Integer) (Math|Float|Floor _returnvalue_4) false true 2) (Utilities|Text|ToText(Integer) (Math|Float|Floor (Math|Float|%(Float) _returnvalue_4 6e+01)) false true 2))))