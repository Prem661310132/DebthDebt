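; AC_Inventory is an inventory component that stores items as rotatable shapes on a 2D grid, including items gained from fishing.
; Inventory maps grid positions to items, while InventoryState tracks each cell's occupancy, built at BeginPlay and updated on add or remove.
; Fishing additions try four rotations, scanning for the first slot where the shape fits.
; It also opens and closes UMG_Inventory, with a scaled variant for the fishmonger, switching cursor and input mode.
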(event Custom|UseInventory
  (bind _returnvalue (Game|GetPlayerController 0))
  (bind _returnvalue_2 (Game|GetPlayerController 0))
  (Variables|Default|GetAS_UMG_inventory
    (:then
      (Widget|RemovefromParent (Variables|Default|GetAS_UMG_inventory))
      (Audio|PlaySound2D "/Game/Sound/SFX/CloseInventorySFX.CloseInventorySFX" 1.0 1.0 0.0 0 0)
      (Variables|Default|SetAS_UMG_inventory 0)
      (Variables|/Script/Engine.PlayerController|SetbShowMouseCursor _returnvalue false)
      (Input|SetInputModeGameOnly _returnvalue false))
    (:else
      (Audio|PlaySound2D "/Game/Sound/SFX/OpenInventorySFX.OpenInventorySFX" 1.0 1.0 0.0 0 0)
      (bind _returnvalue_3 (UserInterface|CreateWidget "/Game/Inventory/IV_Widget/UMG_Inventory.UMG_Inventory_C" 0 (Variables|Default|GetInventory) (Variables|Default|GetInventorySize) (Variables|Default|GetInventoryWidth) self))
      (bind _output_get (Variables|Default|SetAS_UMG_inventory _returnvalue_3))
      (UserInterface|Viewport|AddtoViewport _output_get 0)
      (Variables|/Script/Engine.PlayerController|SetbShowMouseCursor _returnvalue_2 true)
      (Input|SetInputModeGameandUI _returnvalue_2 0 "DoNotLock" true false))))

(event Custom|OpenInventoryInFishmonger
  (bind _returnvalue (Game|GetPlayerController 0))
  (bind _returnvalue_2 (UserInterface|CreateWidget "/Game/Inventory/IV_Widget/UMG_Inventory.UMG_Inventory_C" 0 (Variables|Default|GetInventory) (Variables|Default|GetInventorySize) (Variables|Default|GetInventoryWidth) self))
  (bind _output_get (Variables|Default|SetAS_UMG_inventory _returnvalue_2))
  (Class|CanvasPanelSlot|SetPosition (Class|WidgetLayoutLibrary|SlotasCanvasSlot (Variables|/Game/Inventory/IV_Widget/UMG_Inventory.UMG_Inventory_C|GetUMG_Grid _output_get)) "(X=0.000000,Y=0.000000)")
  (Widget|Transform|SetRenderScale _output_get "(X=0.900000,Y=0.900000)")
  (UserInterface|Viewport|AddtoViewport _output_get 0)
  (Variables|/Script/Engine.PlayerController|SetbShowMouseCursor _returnvalue true)
  (Input|SetInputModeGameandUI _returnvalue 0 "DoNotLock" true false))

(event Custom|ExitFishmongerInventory
  (Widget|RemovefromParent (Variables|Default|GetAS_UMG_inventory))
  (Variables|Default|SetAS_UMG_inventory 0)
  (Input|SetInputModeGameandUI (Game|GetPlayerController 0) 0 "DoNotLock" true false))

(event Custom|ClosedInventoryBeforeInteract
  (bind _returnvalue (Game|GetPlayerController 0))
  (Variables|Default|GetAS_UMG_inventory
    (:then
      (Widget|RemovefromParent (Variables|Default|GetAS_UMG_inventory))
      (Audio|PlaySound2D "/Game/Sound/SFX/CloseInventorySFX.CloseInventorySFX" 1.0 1.0 0.0 0 0)
      (Variables|Default|SetAS_UMG_inventory 0)
      (Variables|/Script/Engine.PlayerController|SetbShowMouseCursor _returnvalue false)
      (Input|SetInputModeGameOnly _returnvalue false))
    (:else)))

(event EventBeginPlay
  (State|DefaultInventoryState))

(fn DefaultInventoryState
  (for _index (range 0 (- (Variables|Default|GetInventorySize) 1))
    (Utilities|Map|Add (Variables|Default|GetInventoryState) (Math|Vector2D|MakeVector2D (LocalVariables|GetL-GridX) (LocalVariables|GetL-GridY)) false)
    (if (== (LocalVariables|GetL-GridX) (- (Variables|Default|GetInventoryWidth) 1))
      (LocalVariables|SetL-GridX 0.0)
      (Math|Float|IncrementFloat (LocalVariables|GetL-GridY))
      (else
        (Math|Float|IncrementFloat (LocalVariables|GetL-GridX)))))
  (bind _keys (Utilities|Map|Keys (Variables|Default|GetInventory)))
  (for _array_element _keys
    (State|AddtoState (.Value (Utilities|Map|Find (Variables|Default|GetInventory) _array_element)) _array_element)))

(fn AddtoState
  (params (ST_Item :type ST%20Item%20Structure%20%28by%20ref%29) (Location :type Vector%202D%20Structure))
  (bind (_dataasset _roation) (Utilities|Struct|BreakST_Item ST_Item))
  (for _array_element (Default|GetShape _dataasset _roation)
    (Utilities|Map|Add (Variables|Default|GetInventoryState) (Math|Conversions|ToVector2D(Vector) (Utilities|Struct|MakeIntVector2 (Math|Float|Round (.X (Math|Vector2D|BreakVector2D (+ _array_element Location)))) (Math|Float|Round (.Y (Math|Vector2D|BreakVector2D (+ _array_element Location)))))) true)))

(fn AddtoInventory
  (params (Key :type Vector%202D%20Structure%20%28by%20ref%29) (Value :type ST%20Item%20Structure%20%28by%20ref%29) (ModifyState :type Boolean))
  (Utilities|Map|Add (Variables|Default|GetInventory) Key Value)
  (if ModifyState
    (State|AddtoState Value Key)))

(fn RemovefromInventory
  (params (Key :type Vector%202D%20Structure) (ModifyState :type Boolean))
  (Utilities|FlowControl|Sequence
    (:then_0
      (if ModifyState
        (State|RemovefromState (.Value (Utilities|Map|Find (Variables|Default|GetInventory) Key)) Key)))
    (:then_1
      (Utilities|Map|Remove (Variables|Default|GetInventory) Key))))

(fn WhereShapeFit
  (params (Shape :type Array%20of%20Vector%202D%20Structures))
  (bind _inventorysize (Variables|Default|GetInventorySize))
  (bind _inventorywidth (Variables|Default|GetInventoryWidth))
  (bind _returnvalue (/ _inventorysize _inventorywidth))
  (for _index (range 0 (- (Variables|Default|GetInventorySize) 1))
    (for _index_2 (range 0 (- (Variables|Default|GetInventoryWidth) 1))
      (LocalVariables|SetL-EmptySlot (Math|Vector2D|MakeVector2D (Math|Conversions|ToFloat(Integer) _index_2) (Math|Conversions|ToFloat(Integer) _index)))
      (bind _array_element (Utilities|Array|ForEachLoopwithBreak Shape :!label _label)
        (:LoopBody
          (if (or (not (Math|Boolean|ANDBoolean (>= (Math|Float|Round (.X (Math|Vector2D|BreakVector2D (+ (LocalVariables|GetL-EmptySlot) _array_element)))) 0) (< (Math|Float|Round (.X (Math|Vector2D|BreakVector2D (+ (LocalVariables|GetL-EmptySlot) _array_element)))) (Variables|Default|GetInventoryWidth)) (>= (Math|Float|Round (.Y (Math|Vector2D|BreakVector2D (+ (LocalVariables|GetL-EmptySlot) _array_element)))) 0) (< (Math|Float|Round (.Y (Math|Vector2D|BreakVector2D (+ (LocalVariables|GetL-EmptySlot) _array_element)))) _returnvalue))) (Math|Boolean|ANDBoolean (< (Math|Float|Round (.X (Math|Vector2D|BreakVector2D (+ (LocalVariables|GetL-EmptySlot) _array_element)))) (Variables|Default|GetInventoryWidth)) (< (Math|Float|Round (.Y (Math|Vector2D|BreakVector2D (+ (LocalVariables|GetL-EmptySlot) _array_element)))) _returnvalue) (.Value (Utilities|Map|Find (Variables|Default|GetInventoryState) (Math|Conversions|ToVector2D(Vector) (Utilities|Struct|MakeIntVector2 (Math|Float|Round (.X (Math|Vector2D|BreakVector2D (+ (LocalVariables|GetL-EmptySlot) _array_element)))) (Math|Float|Round (.Y (Math|Vector2D|BreakVector2D (+ (LocalVariables|GetL-EmptySlot) _array_element))))))))))
            (LocalVariables|SetL-Failed true)
            (goto _label Break)))
        (:Completed
          (if (LocalVariables|GetL-Failed)
            (LocalVariables|SetL-Failed false)
            (else
              (return true (LocalVariables|GetL-EmptySlot))))))))
  (return false ""))

(fn RemovefromState
  (params (ST_Item :type ST%20Item%20Structure%20%28by%20ref%29) (Location :type Vector%202D%20Structure))
  (bind (_dataasset _roation) (Utilities|Struct|BreakST_Item ST_Item))
  (for _array_element (Default|GetShape _dataasset _roation)
    (Utilities|Map|Add (Variables|Default|GetInventoryState) (+ _array_element Location) false)))

(fn AddItemfromFishing
  (params (ItemStructure :type ST%20Item%20Structure))
  (LocalVariables|SetL-ItemStucture ItemStructure)
  (Utilities|FlowControl|Sequence
    (:then_0
      (bind _success (Manage|CheckRotationFit (LocalVariables|GetL-ItemStucture) 0.0))
      (if _success
        (Development|PrintString "AddFromFishingSuccess" true true "(R=0.073908,G=1.000000,B=0.192358,A=1.000000)" :!label _label)
        (return true)))
    (:then_1
      (bind _success_2 (Manage|CheckRotationFit (LocalVariables|GetL-ItemStucture) 9e+01))
      (if _success_2
        (goto _label)))
    (:then_2
      (bind _success_3 (Manage|CheckRotationFit (LocalVariables|GetL-ItemStucture) 1.8e+02))
      (if _success_3
        (goto _label)))
    (:then_3
      (bind _success_4 (Manage|CheckRotationFit (LocalVariables|GetL-ItemStucture) 2.7e+02))
      (if _success_4
        (goto _label)))
    (:then_4
      (Development|PrintString "AddFromFishingFailed" true true "(R=1.000000,G=0.017938,B=0.000000,A=1.000000)")
      (return false))))

(fn CheckRotationFit
  (params (Structure :type ST%20Item%20Structure) (Rotation :type Float%20%28double-precision%29))
  (bind _dataasset (Utilities|Struct|BreakST_Item Structure))
  (bind _defaultshape (Default|GetShape _dataasset Rotation))
  (bind (_returnvalue _validkey) (Condition|WhereShapeFit _defaultshape))
  (if _returnvalue
    (Inventory|AddtoInventory _validkey (Utilities|Struct|MakeST_Item (.DataAsset (Utilities|Struct|BreakST_Item Structure)) Rotation) true)
    (return true)
    (else
      (return false))))

(fn GetEffectiveItemSize
  (params (ItemSize :type Vector%202D%20Structure) (IsRotated :type Boolean))
  (bind (_x _y) (Math|Vector2D|BreakVector2D ItemSize))
  (bind _returnvalue (Math|Float|Round _y))
  (bind _returnvalue_2 (Math|Float|Round _x))
  (return (Math|Integer|SelectInt _returnvalue _returnvalue_2 IsRotated) (Math|Integer|SelectInt _returnvalue_2 _returnvalue IsRotated)))