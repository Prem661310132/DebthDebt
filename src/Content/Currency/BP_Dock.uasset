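; Dock actor where the player ship parks to buy upgrades, unlock fishing rods or end the day.
; Box overlap shows a dock-zone widget, and docking either timeline-lerps or teleports the ship to the parking spot.
; It then opens WBP_DockMenu, binds its dispatchers and blends the camera to the dock until undocking.
; Purchases charge the player's money manager, update boatyard or fishmonger buttons and prices, and play groans on failure.
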(event OnComponentBeginOverlap(Box)
  (params (OverlappedComponent :type Primitive%20Component%20Object%20Reference) (OtherActor :type Actor%20Object%20Reference) (OtherComp :type Primitive%20Component%20Object%20Reference) (OtherBodyIndex :type Integer) (bFromSweep :type Boolean) (SweepResult :type Hit%20Result%20Structure%20%28by%20ref%29))
  (bind _asbp_player_ship_character (Utilities|Casting|CastToBP_PlayerShipCharacter OtherActor))
  (Variables|Default|SetAs%20BP%20Player _asbp_player_ship_character)
  (bind _returnvalue (UserInterface|CreateWidget "/Game/Currency/UMG_DockZone.UMG_DockZone_C"))
  (bind _output_get (Variables|Default|SetDockzone _returnvalue))
  (UserInterface|Viewport|AddtoViewport _output_get 0)
  (Default|Doodle _output_get))

(event OnComponentEndOverlap(Box)
  (params (OverlappedComponent :type Primitive%20Component%20Object%20Reference) (OtherActor :type Actor%20Object%20Reference) (OtherComp :type Primitive%20Component%20Object%20Reference) (OtherBodyIndex :type Integer))
  (Utilities|IsValid (Variables|Default|GetDockzone)
    (:Is%20Valid
      (Widget|SetVisibility (Variables|Default|GetDockzone) "Hidden"))))

(event Custom|Event_UnlockMangroveRod
  (bind _as_bp_player (Variables|Default|GetAs%20BP%20Player))
  (bind _dockui_ref (Variables|Default|GetDockUI_Ref))
  ;[0.15 0.15 0.15 0.5] UnlockRod
  (if (Variables|/Game/ThirdPerson/Blueprints/BP_PlayerShipCharacter.BP_PlayerShipCharacter_C|GetHasMangroveRod _as_bp_player)
    (Audio|PlaySound2D (Utilities|Set|GetItemByIndex (Variables|Default|GetFishmongerGroan) (Math|Random|RandomIntegerinRange 0 3)) 1.0 1.0 0.0 0 0 :!label _label)
    (else
      (bind _success (Default|RemoveMoney (Variables|/Game/ThirdPerson/Blueprints/BP_PlayerShipCharacter.BP_PlayerShipCharacter_C|GetAC_MoneyManager _as_bp_player) 75))
      (if _success
        (Variables|/Game/ThirdPerson/Blueprints/BP_PlayerShipCharacter.BP_PlayerShipCharacter_C|SetHasMangroveRod (Variables|Default|GetAs%20BP%20Player) true)
        (Audio|PlaySound2D "/Game/Sound/SFX/ToolboxUpgrade.ToolboxUpgrade" 1.0 1.0 0.0 0 0)
        (Variables|/Script/UMG.TextBlock|SetText (Variables|/Game/Currency/WBP_DockMenu.WBP_DockMenu_C|GetMangroveRod_Price _dockui_ref) "Sold")
        (Widget|SetVisibility (Variables|/Game/Currency/WBP_DockMenu.WBP_DockMenu_C|GetBTN_Unlock_MangroveRod _dockui_ref) "Hidden")
        (else
          (goto _label))))))

(event Custom|Event_UpgradeEngine
  (bind _as_bp_player (Variables|Default|GetAs%20BP%20Player))
  (bind _dockui_ref (Variables|Default|GetDockUI_Ref))
  (bind _as_bp_player_2 (Variables|Default|GetAs%20BP%20Player))
  (bind _engineprices (Variables|/Game/ThirdPerson/Blueprints/BP_PlayerShipCharacter.BP_PlayerShipCharacter_C|GetEnginePrices _as_bp_player))
  ;[0.15 0.15 0.15 0.5] Upgrade
  (if (< (Variables|/Game/ThirdPerson/Blueprints/BP_PlayerShipCharacter.BP_PlayerShipCharacter_C|GetEngineTier _as_bp_player) (Utilities|Array|Length _engineprices))
    (bind _success (Default|RemoveMoney (Variables|/Game/ThirdPerson/Blueprints/BP_PlayerShipCharacter.BP_PlayerShipCharacter_C|GetAC_MoneyManager (Variables|Default|GetAs%20BP%20Player)) (Utilities|Array|Get(acopy) _engineprices (Variables|/Game/ThirdPerson/Blueprints/BP_PlayerShipCharacter.BP_PlayerShipCharacter_C|GetEngineTier _as_bp_player))))
    (if _success
      (Default|UpgradeShipEngine (Variables|Default|GetAs%20BP%20Player))
      (Audio|PlaySound2D "/Game/Sound/SFX/BoatEngineUpgrade.BoatEngineUpgrade" 1.0 1.0 0.0 0 0)
      (bind _output_get (Variables|/Game/ThirdPerson/Blueprints/BP_PlayerShipCharacter.BP_PlayerShipCharacter_C|SetEngineTier _as_bp_player_2 (+ (Variables|/Game/ThirdPerson/Blueprints/BP_PlayerShipCharacter.BP_PlayerShipCharacter_C|GetEngineTier _as_bp_player_2) 1)))
      (if (< _output_get (Utilities|Array|Length (Variables|/Game/ThirdPerson/Blueprints/BP_PlayerShipCharacter.BP_PlayerShipCharacter_C|GetEnginePrices (Variables|Default|GetAs%20BP%20Player))))
        (CallFunction|CheckBoatyard)
        (else
          (Variables|/Script/UMG.TextBlock|SetText (Variables|/Game/Currency/WBP_DockMenu.WBP_DockMenu_C|GetEngine_Price _dockui_ref) "Max Tier")
          (Widget|SetVisibility (Variables|/Game/Currency/WBP_DockMenu.WBP_DockMenu_C|GetBTN_Upgrade_Engine _dockui_ref) "Hidden")))
      (else
        (Audio|PlaySound2D (Utilities|Set|GetItemByIndex (Variables|Default|GetSoundShipyardGroan) (Math|Random|RandomIntegerinRange 0 2)) 1.0 1.0 0.0 0 0 :!label _label)))
    (else
      (goto _label))))

(event Custom|EventUnlockAbyssalRod
  (bind _as_bp_player (Variables|Default|GetAs%20BP%20Player))
  (bind _dockui_ref (Variables|Default|GetDockUI_Ref))
  ;[0.15 0.15 0.15 0.5] UnlockRod
  (if (not (Variables|/Game/ThirdPerson/Blueprints/BP_PlayerShipCharacter.BP_PlayerShipCharacter_C|GetHasAbyssalRod _as_bp_player))
    (bind _success (Default|RemoveMoney (Variables|/Game/ThirdPerson/Blueprints/BP_PlayerShipCharacter.BP_PlayerShipCharacter_C|GetAC_MoneyManager _as_bp_player) 150))
    (if _success
      (Variables|/Game/ThirdPerson/Blueprints/BP_PlayerShipCharacter.BP_PlayerShipCharacter_C|SetHasAbyssalRod (Variables|Default|GetAs%20BP%20Player) true)
      (Audio|PlaySound2D "/Game/Sound/SFX/ToolboxUpgrade.ToolboxUpgrade" 1.0 1.0 0.0 0 0)
      (Variables|/Script/UMG.TextBlock|SetText (Variables|/Game/Currency/WBP_DockMenu.WBP_DockMenu_C|GetAbyssalRod_Price _dockui_ref) "Sold")
      (Widget|SetVisibility (Variables|/Game/Currency/WBP_DockMenu.WBP_DockMenu_C|GetBTN_Unlock_AbyssalRod _dockui_ref) "Hidden")
      (else
        (Audio|PlaySound2D (Utilities|Set|GetItemByIndex (Variables|Default|GetFishmongerGroan) (Math|Random|RandomIntegerinRange 0 3)) 1.0 1.0 0.0 0 0)))))

(event Custom|Event_EndDay
  ;[0.15 0.15 0.15 0.5] DockActivity
  (Default|SetRestedDock (Variables|Default|GetAs%20BP_DayManager) self)
  (Default|SkipTime (Variables|Default|GetAs%20BP_DayManager)))

(event Custom|Event_UpgradeStorage
  (bind _as_bp_player (Variables|Default|GetAs%20BP%20Player))
  (bind _dockui_ref (Variables|Default|GetDockUI_Ref))
  (bind _as_bp_player_2 (Variables|Default|GetAs%20BP%20Player))
  (bind _storageprices (Variables|/Game/ThirdPerson/Blueprints/BP_PlayerShipCharacter.BP_PlayerShipCharacter_C|GetStoragePrices _as_bp_player))
  ;[0.15 0.15 0.15 0.5] Upgrade
  (if (< (Variables|/Game/ThirdPerson/Blueprints/BP_PlayerShipCharacter.BP_PlayerShipCharacter_C|GetStorageTier _as_bp_player) (Utilities|Array|Length _storageprices))
    (bind _success (Default|RemoveMoney (Variables|/Game/ThirdPerson/Blueprints/BP_PlayerShipCharacter.BP_PlayerShipCharacter_C|GetAC_MoneyManager (Variables|Default|GetAs%20BP%20Player)) (Utilities|Array|Get(acopy) _storageprices (Variables|/Game/ThirdPerson/Blueprints/BP_PlayerShipCharacter.BP_PlayerShipCharacter_C|GetStorageTier _as_bp_player))))
    (if _success
      (Audio|PlaySound2D "/Game/Sound/SFX/StorageUpgrade.StorageUpgrade" 1.0 1.0 0.0 0 0)
      (Default|UpgradeStorage (Variables|Default|GetAs%20BP%20Player))
      (bind _output_get (Variables|/Game/ThirdPerson/Blueprints/BP_PlayerShipCharacter.BP_PlayerShipCharacter_C|SetStorageTier _as_bp_player_2 (+ (Variables|/Game/ThirdPerson/Blueprints/BP_PlayerShipCharacter.BP_PlayerShipCharacter_C|GetStorageTier _as_bp_player_2) 1)))
      (if (< _output_get (Utilities|Array|Length (Variables|/Game/ThirdPerson/Blueprints/BP_PlayerShipCharacter.BP_PlayerShipCharacter_C|GetStoragePrices (Variables|Default|GetAs%20BP%20Player))))
        (CallFunction|CheckBoatyard)
        (else
          (Variables|/Script/UMG.TextBlock|SetText (Variables|/Game/Currency/WBP_DockMenu.WBP_DockMenu_C|GetStorage_Price _dockui_ref) "Max Tier")
          (Widget|SetVisibility (Variables|/Game/Currency/WBP_DockMenu.WBP_DockMenu_C|GetBTN_Upgrade_Storage _dockui_ref) "Hidden")))
      (else
        (Audio|PlaySound2D (Utilities|Set|GetItemByIndex (Variables|Default|GetSoundShipyardGroan) (Math|Random|RandomIntegerinRange 0 2)) 1.0 1.0 0.0 0 0 :!label _label)))
    (else
      (goto _label))))

(event Custom|Event_UpgradeToolbox
  (bind _as_bp_player (Variables|Default|GetAs%20BP%20Player))
  (bind _dockui_ref (Variables|Default|GetDockUI_Ref))
  (bind _as_bp_player_2 (Variables|Default|GetAs%20BP%20Player))
  (bind _fishingrodtier (Variables|/Game/ThirdPerson/Blueprints/BP_PlayerShipCharacter.BP_PlayerShipCharacter_C|GetFishingRodTier _as_bp_player))
  (bind _fishingrodprices (Variables|/Game/ThirdPerson/Blueprints/BP_PlayerShipCharacter.BP_PlayerShipCharacter_C|GetFishingRodPrices _as_bp_player))
  ;[0.15 0.15 0.15 0.5] Upgrade
  (if (< _fishingrodtier (Utilities|Array|Length _fishingrodprices))
    (bind _success (Default|RemoveMoney (Variables|/Game/ThirdPerson/Blueprints/BP_PlayerShipCharacter.BP_PlayerShipCharacter_C|GetAC_MoneyManager (Variables|Default|GetAs%20BP%20Player)) (Utilities|Array|Get(acopy) _fishingrodprices _fishingrodtier)))
    (if _success
      (Audio|PlaySound2D "/Game/Sound/SFX/ToolboxUpgrade.ToolboxUpgrade" 1.0 1.0 0.0 0 0)
      (Default|UpgradeFishingRod (Variables|Default|GetAs%20BP%20Player))
      (if (< (Variables|/Game/ThirdPerson/Blueprints/BP_PlayerShipCharacter.BP_PlayerShipCharacter_C|GetFishingRodTier _as_bp_player_2) (Utilities|Array|Length (Variables|/Game/ThirdPerson/Blueprints/BP_PlayerShipCharacter.BP_PlayerShipCharacter_C|GetFishingRodPrices _as_bp_player_2)))
        (CallFunction|CheckFishmonger)
        (else
          (Variables|/Script/UMG.TextBlock|SetText (Variables|/Game/Currency/WBP_DockMenu.WBP_DockMenu_C|GetTackleBox_Price _dockui_ref) "Max Tier")
          (Widget|SetVisibility (Variables|/Game/Currency/WBP_DockMenu.WBP_DockMenu_C|GetBTN_Upgrade_Fishing _dockui_ref) "Hidden")))
      (else
        (Audio|PlaySound2D (Utilities|Set|GetItemByIndex (Variables|Default|GetFishmongerGroan) (Math|Random|RandomIntegerinRange 0 3)) 1.0 1.0 0.0 0 0 :!label _label)))
    (else
      (goto _label))))

(event Custom|Event_UndockShip
  (bind _returnvalue (Game|GetPlayerController 0))
  ;[0.15 0.15 0.15 0.5] DockActivity
  (Widget|RemovefromParent (Variables|Default|GetDockUI_Ref))
  (Variables|/Game/ThirdPerson/Blueprints/BP_PlayerShipCharacter.BP_PlayerShipCharacter_C|SetIsDocked (Variables|Default|GetAs%20BP%20Player) false)
  (Variables|/Script/Engine.PlayerController|SetbShowMouseCursor _returnvalue false)
  (Input|SetInputModeGameOnly _returnvalue false)
  (Game|Player|SetViewTargetwithBlend _returnvalue (Variables|Default|GetAs%20BP%20Player) 1.0 "VTBlend_Linear" 0.0 false)
  (Audio|Components|Audio|FadeIn (Variables|/Game/ThirdPerson/Blueprints/BP_PlayerShipCharacter.BP_PlayerShipCharacter_C|GetMotorSound (Variables|Default|GetAs%20BP%20Player)) 2.0 1.0 0.0 "Linear" :!class /Script/Engine.AudioComponent))

(event Custom|Event_UnlockDeepWaterRod
  (bind _dockui_ref (Variables|Default|GetDockUI_Ref))
  (bind _as_bp_player (Variables|Default|GetAs%20BP%20Player))
  ;[0.15 0.15 0.15 0.5] UnlockRod
  (if (Variables|/Game/ThirdPerson/Blueprints/BP_PlayerShipCharacter.BP_PlayerShipCharacter_C|GetHasDeepWaterRod _as_bp_player)
    (Audio|PlaySound2D (Utilities|Set|GetItemByIndex (Variables|Default|GetFishmongerGroan) (Math|Random|RandomIntegerinRange 0 3)) 1.0 1.0 0.0 0 0 :!label _label)
    (else
      (bind _success (Default|RemoveMoney (Variables|/Game/ThirdPerson/Blueprints/BP_PlayerShipCharacter.BP_PlayerShipCharacter_C|GetAC_MoneyManager _as_bp_player) 100))
      (if _success
        (Variables|/Game/ThirdPerson/Blueprints/BP_PlayerShipCharacter.BP_PlayerShipCharacter_C|SetHasDeepWaterRod (Variables|Default|GetAs%20BP%20Player) true)
        (Audio|PlaySound2D "/Game/Sound/SFX/ToolboxUpgrade.ToolboxUpgrade" 1.0 1.0 0.0 0 0)
        (Variables|/Script/UMG.TextBlock|SetText (Variables|/Game/Currency/WBP_DockMenu.WBP_DockMenu_C|GetDeepWaterRod_Price _dockui_ref) "Sold")
        (Widget|SetVisibility (Variables|/Game/Currency/WBP_DockMenu.WBP_DockMenu_C|GetBTN_Unlock_DeepWaterRod _dockui_ref) "Hidden")
        (else
          (goto _label))))))

(event Custom|InstantDocking
  (bind _returnvalue (Game|GetPlayerController 0))
  (bind _parkingspot (Variables|Default|GetParkingSpot))
  (bind _as_bp_player (Variables|Default|GetAs%20BP%20Player))
  (bind _returnvalue_2 (Transformation|GetWorldTransform _parkingspot))
  ;[0.15 0.15 0.15 0.5] InstantDocking
  (Widget|SetVisibility (Variables|Default|GetDockzone) "Hidden")
  (Variables|/Game/ThirdPerson/Blueprints/BP_PlayerShipCharacter.BP_PlayerShipCharacter_C|SetIsDocked _as_bp_player true)
  (Transformation|SetActorLocationAndRotation _as_bp_player (.location _returnvalue_2) (.rotation _returnvalue_2) false true)
  (bind _returnvalue_3 (UserInterface|CreateWidget "/Game/Currency/WBP_DockMenu.WBP_DockMenu_C" 0 (Variables|Default|GetisALone)))
  (bind _output_get (Variables|Default|SetDockUI_Ref _returnvalue_3))
  (UserInterface|Viewport|AddtoViewport _output_get 0)
  (EventDispatchers|BindEventtoEDUndock _output_get (EventDispatchers|CreateEvent :!event Custom|Event_UndockShip))
  (EventDispatchers|BindEventtoEDUpgradeEngine _output_get (EventDispatchers|CreateEvent :!event Custom|Event_UpgradeEngine))
  (EventDispatchers|BindEventtoEDUpgradeStorage _output_get (EventDispatchers|CreateEvent :!event Custom|Event_UpgradeStorage))
  (EventDispatchers|BindEventtoEDUpgradeToolBox _output_get (EventDispatchers|CreateEvent :!event Custom|Event_UpgradeToolbox))
  (EventDispatchers|BindEventtoEDUnlockDeepWaterRod _output_get (EventDispatchers|CreateEvent :!event Custom|Event_UnlockDeepWaterRod))
  (EventDispatchers|BindEventtoEDUnlockMangroveRod _output_get (EventDispatchers|CreateEvent :!event Custom|Event_UnlockMangroveRod))
  (EventDispatchers|BindEventtoEDCheckFishmonger _output_get (EventDispatchers|CreateEvent :!event Custom|CheckFishmonger))
  (EventDispatchers|BindEventtoEDCheckBoatyard _output_get (EventDispatchers|CreateEvent :!event Custom|CheckBoatyard))
  (EventDispatchers|BindEventtoEDUnlockAbyssalRod _output_get (EventDispatchers|CreateEvent :!event Custom|EventUnlockAbyssalRod))
  (EventDispatchers|BindEventtoEDEndDay _output_get (EventDispatchers|CreateEvent :!event Custom|Event_EndDay))
  (Variables|/Script/Engine.PlayerController|SetbShowMouseCursor _returnvalue true)
  (Input|SetInputModeUIOnly _returnvalue (Variables|Default|GetDockUI_Ref) "DoNotLock" false)
  (Game|Player|SetViewTargetwithBlend _returnvalue self 1.0 "VTBlend_Linear" 0.0 false))

(event Custom|CheckFishmonger
  (bind _as_bp_player (Variables|Default|GetAs%20BP%20Player))
  (bind _dockui_ref (Variables|Default|GetDockUI_Ref))
  (bind _dockui_ref_2 (Variables|Default|GetDockUI_Ref))
  (bind _as_bp_player_2 (Variables|Default|GetAs%20BP%20Player))
  (bind _dockui_ref_3 (Variables|Default|GetDockUI_Ref))
  (bind _dockui_ref_4 (Variables|Default|GetDockUI_Ref))
  ;[0.15 0.15 0.15 0.5] CheckButton
  (Default|UpdateFishmongerPrice (Variables|Default|GetDockUI_Ref) (Utilities|Array|Get(acopy) (Variables|/Game/ThirdPerson/Blueprints/BP_PlayerShipCharacter.BP_PlayerShipCharacter_C|GetFishingRodPrices _as_bp_player_2) (Variables|/Game/ThirdPerson/Blueprints/BP_PlayerShipCharacter.BP_PlayerShipCharacter_C|GetFishingRodTier _as_bp_player_2)) 75 100 150)
  (if (< (Variables|/Game/ThirdPerson/Blueprints/BP_PlayerShipCharacter.BP_PlayerShipCharacter_C|GetFishingRodTier (Variables|Default|GetAs%20BP%20Player)) (Utilities|Array|Length (Variables|/Game/ThirdPerson/Blueprints/BP_PlayerShipCharacter.BP_PlayerShipCharacter_C|GetFishingRodPrices (Variables|Default|GetAs%20BP%20Player))))
    _
    (else
      (Variables|/Script/UMG.TextBlock|SetText (Variables|/Game/Currency/WBP_DockMenu.WBP_DockMenu_C|GetTackleBox_Price _dockui_ref_3) "Max Tier")
      (Widget|SetVisibility (Variables|/Game/Currency/WBP_DockMenu.WBP_DockMenu_C|GetBTN_Upgrade_Fishing _dockui_ref_3) "Hidden")))
  (if (Variables|/Game/ThirdPerson/Blueprints/BP_PlayerShipCharacter.BP_PlayerShipCharacter_C|GetHasMangroveRod _as_bp_player)
    (Variables|/Script/UMG.TextBlock|SetText (Variables|/Game/Currency/WBP_DockMenu.WBP_DockMenu_C|GetMangroveRod_Price _dockui_ref_4) "Sold")
    (Widget|SetVisibility (Variables|/Game/Currency/WBP_DockMenu.WBP_DockMenu_C|GetBTN_Unlock_MangroveRod _dockui_ref_4) "Hidden"))
  (if (Variables|/Game/ThirdPerson/Blueprints/BP_PlayerShipCharacter.BP_PlayerShipCharacter_C|GetHasDeepWaterRod _as_bp_player)
    (Variables|/Script/UMG.TextBlock|SetText (Variables|/Game/Currency/WBP_DockMenu.WBP_DockMenu_C|GetDeepWaterRod_Price _dockui_ref_2) "Sold")
    (Widget|SetVisibility (Variables|/Game/Currency/WBP_DockMenu.WBP_DockMenu_C|GetBTN_Unlock_DeepWaterRod _dockui_ref_2) "Hidden"))
  (if (Variables|/Game/ThirdPerson/Blueprints/BP_PlayerShipCharacter.BP_PlayerShipCharacter_C|GetHasAbyssalRod _as_bp_player)
    (Variables|/Script/UMG.TextBlock|SetText (Variables|/Game/Currency/WBP_DockMenu.WBP_DockMenu_C|GetAbyssalRod_Price _dockui_ref) "Sold")
    (Widget|SetVisibility (Variables|/Game/Currency/WBP_DockMenu.WBP_DockMenu_C|GetBTN_Unlock_AbyssalRod _dockui_ref) "Hidden")))

(event Custom|CheckBoatyard
  (bind _as_bp_player (Variables|Default|GetAs%20BP%20Player))
  (bind _as_bp_player_2 (Variables|Default|GetAs%20BP%20Player))
  (bind _dockui_ref (Variables|Default|GetDockUI_Ref))
  (bind _dockui_ref_2 (Variables|Default|GetDockUI_Ref))
  ;[0.15 0.15 0.15 0.5] CheckButton
  (Default|UpdateShipwrightPrice (Variables|Default|GetDockUI_Ref) (Utilities|Array|Get(acopy) (Variables|/Game/ThirdPerson/Blueprints/BP_PlayerShipCharacter.BP_PlayerShipCharacter_C|GetStoragePrices _as_bp_player) (Variables|/Game/ThirdPerson/Blueprints/BP_PlayerShipCharacter.BP_PlayerShipCharacter_C|GetStorageTier _as_bp_player)) (Utilities|Array|Get(acopy) (Variables|/Game/ThirdPerson/Blueprints/BP_PlayerShipCharacter.BP_PlayerShipCharacter_C|GetEnginePrices _as_bp_player_2) (Variables|/Game/ThirdPerson/Blueprints/BP_PlayerShipCharacter.BP_PlayerShipCharacter_C|GetEngineTier _as_bp_player_2)))
  (if (< (Variables|/Game/ThirdPerson/Blueprints/BP_PlayerShipCharacter.BP_PlayerShipCharacter_C|GetEngineTier (Variables|Default|GetAs%20BP%20Player)) (Utilities|Array|Length (Variables|/Game/ThirdPerson/Blueprints/BP_PlayerShipCharacter.BP_PlayerShipCharacter_C|GetEnginePrices (Variables|Default|GetAs%20BP%20Player))))
    _
    (else
      (Variables|/Script/UMG.TextBlock|SetText (Variables|/Game/Currency/WBP_DockMenu.WBP_DockMenu_C|GetEngine_Price _dockui_ref) "Max Tier")
      (Widget|SetVisibility (Variables|/Game/Currency/WBP_DockMenu.WBP_DockMenu_C|GetBTN_Upgrade_Engine _dockui_ref) "Hidden")))
  (if (not (< (Variables|/Game/ThirdPerson/Blueprints/BP_PlayerShipCharacter.BP_PlayerShipCharacter_C|GetStorageTier (Variables|Default|GetAs%20BP%20Player)) (Utilities|Array|Length (Variables|/Game/ThirdPerson/Blueprints/BP_PlayerShipCharacter.BP_PlayerShipCharacter_C|GetStoragePrices (Variables|Default|GetAs%20BP%20Player)))))
    (Variables|/Script/UMG.TextBlock|SetText (Variables|/Game/Currency/WBP_DockMenu.WBP_DockMenu_C|GetStorage_Price _dockui_ref_2) "Max Tier")
    (Widget|SetVisibility (Variables|/Game/Currency/WBP_DockMenu.WBP_DockMenu_C|GetBTN_Upgrade_Storage _dockui_ref_2) "Hidden")))

(event EventStartDocking
  (bind _returnvalue (Game|GetPlayerController 0))
  (bind _as_bp_player (Variables|Default|GetAs%20BP%20Player))
  (bind _parkingspot (Variables|Default|GetParkingSpot))
  (bind _returnvalue_2 (Transformation|GetWorldTransform _parkingspot))
  (bind _rootcomponent (Variables|/Script/Engine.Actor|GetRootComponent _as_bp_player))
  (bind _returnvalue_3 (Transformation|GetWorldTransform _rootcomponent))
  (Widget|SetVisibility (Variables|Default|GetDockzone) "Hidden")
  (Variables|Default|SetStartLocation (.location _returnvalue_3))
  (Variables|Default|SetStartRotation (.rotation _returnvalue_3))
  (bind _alpha (Timeline|DockingTimeline PlayFromStart)
    (:Update
      (Transformation|SetActorLocationAndRotation (Variables|Default|GetAs%20BP%20Player) (Math|Vector|Lerp(Vector) (Variables|Default|GetStartLocation) (.location _returnvalue_2) _alpha) (Math|Rotator|Lerp(Rotator) (Variables|Default|GetStartRotation) (.rotation _returnvalue_2) _alpha)))
    (:Finished
      (Audio|PlaySound2D "/Game/Sound/SFX/Rope.Rope" 1.0 1.0 0.0 0 0)
      (bind _returnvalue_4 (UserInterface|CreateWidget "/Game/Currency/WBP_DockMenu.WBP_DockMenu_C" 0 (Variables|Default|GetisALone)))
      (bind _output_get (Variables|Default|SetDockUI_Ref _returnvalue_4))
      (UserInterface|Viewport|AddtoViewport _output_get 0)
      (EventDispatchers|BindEventtoEDUndock _output_get (EventDispatchers|CreateEvent :!event Custom|Event_UndockShip))
      (EventDispatchers|BindEventtoEDUpgradeEngine _output_get (EventDispatchers|CreateEvent :!event Custom|Event_UpgradeEngine))
      (EventDispatchers|BindEventtoEDUpgradeStorage _output_get (EventDispatchers|CreateEvent :!event Custom|Event_UpgradeStorage))
      (EventDispatchers|BindEventtoEDUpgradeToolBox _output_get (EventDispatchers|CreateEvent :!event Custom|Event_UpgradeToolbox))
      (EventDispatchers|BindEventtoEDUnlockDeepWaterRod _output_get (EventDispatchers|CreateEvent :!event Custom|Event_UnlockDeepWaterRod))
      (EventDispatchers|BindEventtoEDUnlockMangroveRod _output_get (EventDispatchers|CreateEvent :!event Custom|Event_UnlockMangroveRod))
      (EventDispatchers|BindEventtoEDCheckFishmonger _output_get (EventDispatchers|CreateEvent :!event Custom|CheckFishmonger))
      (EventDispatchers|BindEventtoEDCheckBoatyard _output_get (EventDispatchers|CreateEvent :!event Custom|CheckBoatyard))
      (EventDispatchers|BindEventtoEDUnlockAbyssalRod _output_get (EventDispatchers|CreateEvent :!event Custom|EventUnlockAbyssalRod))
      (EventDispatchers|BindEventtoEDEndDay _output_get (EventDispatchers|CreateEvent :!event Custom|Event_EndDay))
      (Variables|/Script/Engine.PlayerController|SetbShowMouseCursor _returnvalue true)
      (Input|SetInputModeUIOnly _returnvalue (Variables|Default|GetDockUI_Ref) "DoNotLock" false)
      (Game|Player|SetViewTargetwithBlend _returnvalue self 1.0 "VTBlend_Linear" 0.0 false))))

(fn ConstructionScript)