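; AC_MoneyManager is a currency component that tracks a CurrentMoney balance.
; AddMoney increases the balance, while RemoveMoney subtracts only when the balance covers the amount and returns whether it succeeded.
; Both broadcast OnMoneyChanged with the new balance after a change, so listeners can react without polling.
; HasEnoughMoney offers a read-only affordability check, and the event graph holds no active logic.
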(event EventBeginPlay)

(event EventTick
  (params (DeltaSeconds :type Float%20%28single-precision%29)))

(fn AddMoney
  (params (Amount :type Integer))
  (bind _output_get (Variables|Default|SetCurrentMoney (+ Amount (Variables|Default|GetCurrentMoney))))
  (Default|CallOnMoneyChanged _output_get)
  (return))

(fn RemoveMoney
  (params (Amount :type Integer))
  (if (>= (Variables|Default|GetCurrentMoney) Amount)
    (bind _output_get (Variables|Default|SetCurrentMoney (- (Variables|Default|GetCurrentMoney) Amount)))
    (Default|CallOnMoneyChanged _output_get)
    (return true)
    (else
      (return false))))

(fn HasEnoughMoney
  (params (Amount :type Integer))
  (return (>= (Variables|Default|GetCurrentMoney) Amount)))